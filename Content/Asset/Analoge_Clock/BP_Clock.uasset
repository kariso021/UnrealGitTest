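; BP_Clock is an analog clock actor that shows the real current system time.
; From BeginPlay, a Delay loop reads Now every second and sets each hand's relative pitch from the hour, minute and second.
; The hour angle includes a minute offset for gradual movement.
; The component names are swapped relative to the math: ClockMinutesHand receives the hour angle and ClockHourHand the minute angle.
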(event `self.ReceiveBeginPlay`
  (bind (_year _month _day _hour _minute _second) (`KismetMathLibrary.BreakDateTime` (`KismetMathLibrary.Now`)))
  (`SceneComponent.K2_SetRelativeRotation` (`self.Clock_Minutes_Hand`) (`KismetMathLibrary.MakeRotator` 0.0 (+ (`KismetMathLibrary.Conv_IntToDouble` (* _hour -30)) (/ (`KismetMathLibrary.Conv_IntToDouble` _minute) -2.0))) false false :!label _label)
  (`SceneComponent.K2_SetRelativeRotation` (`self.Clock_Hour_Hand`) (`KismetMathLibrary.MakeRotator` 0.0 (`KismetMathLibrary.Conv_IntToDouble` (* _minute -6))) false false)
  (`SceneComponent.K2_SetRelativeRotation` (`self.Clock_Seconds_Hand`) (`KismetMathLibrary.MakeRotator` 0.0 (`KismetMathLibrary.Conv_IntToDouble` (* _second -6))) false false)
  (`KismetSystemLibrary.Delay` 1.0)
  (goto _label))

(fn `UserConstructionScript`)