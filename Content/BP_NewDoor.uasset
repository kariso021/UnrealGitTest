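; A double door actor that swings its two leaves open or closed when OpenDoor fires while the overlap flag is set.
; Actor begin and end overlap set and clear that flag, with no check on which actor overlaps.
; Each leaf has its own FlipFlop and timeline, which alternately plays and reverses to lerp that door's relative yaw, turning the leaves in opposite directions.
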(event `OpenDoor`
  (if (`self.checkInt`)
    (`|ExecutionSequence`
      (:`then_0`
        (`/Engine/EditorBlueprintResources/StandardMacros.FlipFlop`
          (:`A`
            (bind (_direction _door_open) (`Timeline|OpenDoorTimeline` :!via `PlayFromStart` :!label _label)
              (:`Update`
                (`SceneComponent.K2_SetRelativeRotation` (`self.door2`) (`KismetMathLibrary.MakeRotator` 0.0 0.0 (`KismetMathLibrary.Lerp` 180.0 90.0 _door_open)) false false))))
          (:`B`
            (goto _label :!via `Reverse`))))
      (:`then_1`
        (`/Engine/EditorBlueprintResources/StandardMacros.FlipFlop`
          (:`A`
            (bind (_direction_2 _door_open_2) (`Timeline|Timeline` :!via `PlayFromStart` :!label _label_2)
              (:`Update`
                (`SceneComponent.K2_SetRelativeRotation` (`self.door1`) (`KismetMathLibrary.MakeRotator` 0.0 0.0 (`KismetMathLibrary.Lerp` 0.0 90.0 _door_open_2)) false false))))
          (:`B`
            (goto _label_2 :!via `Reverse`)))))))

(event `self.ReceiveActorBeginOverlap`
  (params (OtherActor :type "Actor Object Reference"))
  (set `self.checkInt` true))

(event `self.ReceiveActorEndOverlap`
  (params (OtherActor :type "Actor Object Reference"))
  (set `self.checkInt` false))

(fn `UserConstructionScript`)