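; Door actor Blueprint that swings its static mesh open and closed around the yaw axis.
; BeginPlay caches the mesh's world rotation, and a timeline's ZAxis track supplies a yaw offset that is combined with that rotation on each update.
; OpenDoor prints a debug string and plays the timeline, while CloseDoor reverses it.
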(event `self.ReceiveBeginPlay`
  (set `self.Default Rotation` (`SceneComponent.K2_GetComponentRotation` (`self.StaticMeshComponent`))))

(event `OpenDoor`
  (`KismetSystemLibrary.PrintString` "Open")
  (bind (_direction _zaxis) (`Timeline|Door Timeline` :!label _label)
    (:`Update`
      (`SceneComponent.K2_SetWorldRotation` (`self.StaticMeshComponent`) (`KismetMathLibrary.ComposeRotators` (`KismetMathLibrary.MakeRotator` 0.0 0.0 _zaxis) (`self.Default Rotation`)) false false))))

(event `Close Door`
  (goto _label :!via `Reverse`))

(fn `UserConstructionScript`)