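; Keypad-locked sliding door that opens for the first-person character once IsCorrect is true.
; While locked, entering the trigger box shows the password widget with the mouse cursor and Game-and-UI input.
; Once unlocked, entering calls ChangeLight on Lightt, adds the KEY widget, hides the cursor and slides the mesh between hardcoded relative positions via a Timeline.
; Leaving the box reverses the Timeline.
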(event `self.Box.OnComponentBeginOverlap`
  (params (OverlappedComponent :type "PrimitiveComponent Object Reference") (OtherActor :type "Actor Object Reference") (OtherComp :type "PrimitiveComponent Object Reference") (OtherBodyIndex :type Integer) (bFromSweep :type Boolean) (SweepResult :type "HitResult Structure (by ref)"))
  (bind _returnvalue (`GameplayStatics.GetPlayerController` 0))
  (cast `/Game/SpotlightReveal/Blueprints/FirstPersonCharacter` OtherActor)
  (if (`self.isCorrect`)
    (`/Game/BP/BP_Light.ChangeLight` (`self.Lightt`))
    (bind _returnvalue_2 (`|CreateWidget` "/Game/BP/KEY.KEY_C"))
    (`UserWidget.AddToViewport` _returnvalue_2 0)
    (set `PlayerController.bShowMouseCursor` false _returnvalue)
    (bind (_direction _track) (`Timeline|Timeline` :!label _label)
      (:`Update`
        (`SceneComponent.K2_SetRelativeLocation` (`self.StaticMeshComponent`) (`KismetMathLibrary.VLerp` (970.0 430.0 0.0) (970.0 280.0 0.0) _track) false false)))
    (else
      (bind _returnvalue_3 (`|CreateWidget` "/Game/BP/WD_PasswordWidget.WD_PasswordWidget_C"))
      (`UserWidget.AddToViewport` _returnvalue_3 0)
      (set `PlayerController.bShowMouseCursor` true _returnvalue)
      (`WidgetBlueprintLibrary.SetInputMode_GameAndUIEx` _returnvalue _returnvalue_3))))

(event `self.Box.OnComponentEndOverlap`
  (params (OverlappedComponent :type "PrimitiveComponent Object Reference") (OtherActor :type "Actor Object Reference") (OtherComp :type "PrimitiveComponent Object Reference") (OtherBodyIndex :type Integer))
  (cast `/Game/SpotlightReveal/Blueprints/FirstPersonCharacter` OtherActor)
  (goto _label :!via `Reverse`))

(fn `UserConstructionScript`)