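; BP_TableandImage is an interactable table actor that, when revealed, switches the player's view to itself and opens a table UI.
; Reveal blends the camera to the actor, blocks move and look input, adds a WZ_Table widget to the viewport and shows the mouse cursor.
; Overlap events toggle a CheckClose flag to track proximity, while nothing in this graph calls Reveal or restores player control.
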(event `Reveal`
  (bind _returnvalue (`GameplayStatics.GetPlayerController` 0))
  (`PlayerController.SetViewTargetWithBlend` (`GameplayStatics.GetPlayerController` 0) self 2.0 "VTBlend_Linear" 0.0 false)
  (`Controller.SetIgnoreMoveInput` _returnvalue true)
  (`Controller.SetIgnoreLookInput` _returnvalue true)
  (bind _returnvalue_2 (`|CreateWidget` "/Game/WZ_Table.WZ_Table_C"))
  (`UserWidget.AddToViewport` _returnvalue_2 0)
  (set `PlayerController.bShowMouseCursor` true (`GameplayStatics.GetPlayerController` 0)))

(event `self.ReceiveActorBeginOverlap`
  (params (OtherActor :type "Actor Object Reference"))
  (set `self.CheckClose` true))

(event `self.ReceiveActorEndOverlap`
  (params (OtherActor :type "Actor Object Reference"))
  (set `self.CheckClose` false))

(fn `UserConstructionScript`)