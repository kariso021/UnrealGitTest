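; Blueprint function library that feeds a spotlight's cone into the MPC_SpotlightReveal parameter collection, presumably for materials that reveal surfaces under the light.
; It writes attenuation and start position, then traces forward on Visibility to set the end point at the hit or at full range.
; Cone radius comes from that distance and the tangent of the outer cone angle.
; A hidden light collapses the end point to the start and zeroes the radius.
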(fn `SpotlightReveal`
  (params (Spotlight :type "SpotLightComponent Object Reference"))
  (bind _returnvalue (`SceneComponent.K2_GetComponentLocation` Spotlight))
  (bind _attenuationradius (`LocalLightComponent.AttenuationRadius` Spotlight))
  (bind _attenuationradius_2 (`LocalLightComponent.AttenuationRadius` Spotlight))
  (bind _returnvalue_2 (`KismetMathLibrary.DegTan` (`SpotLightComponent.OuterConeAngle` Spotlight)))
  (bind _returnvalue_3 (+ _returnvalue (* (`SceneComponent.GetForwardVector` Spotlight) _attenuationradius)))
  (`KismetMaterialLibrary.SetScalarParameterValue` null "/Game/SpotlightReveal/Materials/MPC_SpotlightReveal.MPC_SpotlightReveal" "Attenuation" _attenuationradius)
  (`KismetMaterialLibrary.SetVectorParameterValue` null "/Game/SpotlightReveal/Materials/MPC_SpotlightReveal.MPC_SpotlightReveal" "StartSpot" (`KismetMathLibrary.Conv_VectorToLinearColor` _returnvalue))
  (if (`SceneComponent.IsVisible` Spotlight)
    (bind (_outhit _returnvalue_4) (`KismetSystemLibrary.LineTraceSingle` null _returnvalue _returnvalue_3 "TraceTypeQuery1"))
    (if _returnvalue_4
      (bind (_bblockinghit _binitialoverlap _time _distance _location _impactpoint) (`GameplayStatics.BreakHitResult` _outhit))
      (`KismetMaterialLibrary.SetVectorParameterValue` null "/Game/SpotlightReveal/Materials/MPC_SpotlightReveal.MPC_SpotlightReveal" "EndSpot" (`KismetMathLibrary.Conv_VectorToLinearColor` _impactpoint))
      (`KismetMaterialLibrary.SetScalarParameterValue` null "/Game/SpotlightReveal/Materials/MPC_SpotlightReveal.MPC_SpotlightReveal" "Radius" (* (`KismetMathLibrary.FClamp` (`KismetMathLibrary.VSize` (- _impactpoint (`SceneComponent.K2_GetComponentLocation` Spotlight))) 0.0 _attenuationradius_2) _returnvalue_2))
      (else
        (`KismetMaterialLibrary.SetVectorParameterValue` null "/Game/SpotlightReveal/Materials/MPC_SpotlightReveal.MPC_SpotlightReveal" "EndSpot" (`KismetMathLibrary.Conv_VectorToLinearColor` _returnvalue_3))
        (`KismetMaterialLibrary.SetScalarParameterValue` null "/Game/SpotlightReveal/Materials/MPC_SpotlightReveal.MPC_SpotlightReveal" "Radius" (* _attenuationradius_2 _returnvalue_2))))
    (else
      (`KismetMaterialLibrary.SetVectorParameterValue` null "/Game/SpotlightReveal/Materials/MPC_SpotlightReveal.MPC_SpotlightReveal" "EndSpot" (`KismetMathLibrary.Conv_VectorToLinearColor` (`SceneComponent.K2_GetComponentLocation` Spotlight)))
      (`KismetMaterialLibrary.SetScalarParameterValue` null "/Game/SpotlightReveal/Materials/MPC_SpotlightReveal.MPC_SpotlightReveal" "Radius"))))